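; Player character Blueprint for a platformer with wall running, crouching, sliding, dashing and grappling.
; Timelines drive camera tilt, crouch height and dash FOV, passing values to update functions defined outside this graph, while capsule hits feed wall-run checks.
; The grapple event shows and sizes a cable toward the target.
; It also creates the gameplay HUD and toggles an options menu on Escape, syncing FPS settings.
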(event `Key|Escape`
  (params (Key :type "Key Structure"))
  (bind _returnvalue (`GameplayStatics.GetPlayerController` 0))
  (bind _optionsmenu (`self.OptionsMenu`))
  (bind _optionsmenu_2 (`self.OptionsMenu`))
  ;[0 0.1778 0.7927] Settings
  (:`Pressed`
    (`/Engine/EditorBlueprintResources/StandardMacros.FlipFlop`
      (:`A`
        (bind _returnvalue_2 (`|CreateWidget` "/Game/UI/Menu.Menu_C" _returnvalue))
        (bind _output_get (set `self.OptionsMenu` _returnvalue_2))
        (`UserWidget.AddToViewport` _output_get 0)
        (`WidgetBlueprintLibrary.SetInputMode_GameAndUIEx` _returnvalue null)
        (set `PlayerController.bShowMouseCursor` true _returnvalue)
        (set `/Game/UI/Menu.bShowFPS` (`self.ShowFPS`) _optionsmenu_2)
        (set `/Game/UI/Menu.FPSLimit` (`self.FPSLimitPre`) _optionsmenu_2))
      (:`B`
        (bind _output_get_2 (set `self.ShowFPS` (`/Game/UI/Menu.bShowFPS` _optionsmenu)))
        (set `self.FPSLimitPre` (`/Game/UI/Menu.FPSLimit` _optionsmenu))
        (`/Game/UI/GameplayUI.OnChangeShowFPS` (`self.GameplayUI`) _output_get_2)
        (`Widget.RemoveFromParent` _optionsmenu)
        (set `PlayerController.bShowMouseCursor` false _returnvalue)
        (`WidgetBlueprintLibrary.SetInputMode_GameOnly` _returnvalue)))))

(event `self.ReceiveBeginPlay`
  ;[0.5177 0.01349 0] BeginPlay
  (bind _returnvalue (`|CreateWidget` "/Game/UI/GameplayUI.GameplayUI_C" (`GameplayStatics.GetPlayerController` 0)))
  (bind _output_get (set `self.GameplayUI` _returnvalue))
  (`UserWidget.AddToViewport` _output_get 0)
  (`SceneComponent.SetVisibility` (`self.GrappleCable`) false false))

(event `self.CapsuleComponent.OnComponentHit`
  (params (HitComponent :type "PrimitiveComponent Object Reference") (OtherActor :type "Actor Object Reference") (OtherComp :type "PrimitiveComponent Object Reference") (NormalImpulse :type "Vector Structure") (Hit :type "HitResult Structure (by ref)"))
  (`self.CheckWallRunConditions` Hit_ImpactNormal OtherComp))

(event `self.StartCameraTilt`
  ;[0.04236 0.1802 0 1 20] Wall Running Camera Rotation
  (bind (_direction _cameraroll) (`Timeline|Timeline` :!label _label)
    (:`Update`
      (`self.CameraTiltEffectValue` _cameraroll))))

(event `self.EndCameraTilt`
  ;[0.04236 0.1802 0 1 20] Wall Running Camera Rotation
  (goto _label :!via `Reverse`))

(event `self.BeginCrouchEffect`
  ;[0.03672 0.2052 0 1 20] Crouching System
  (bind (_direction _halfheight) (`Timeline|Timeline_0` :!label _label_2)
    (:`Update`
      (`self.UpdateCrouchSystem` _halfheight))))

(event `self.EndCrouchEffect`
  ;[0.03672 0.2052 0 1 20] Crouching System
  (goto _label_2 :!via `Reverse`))

(event `self.GrappleRopeSystem`
  (params (Grappling :type Boolean))
  (bind _grapplecable (`self.GrappleCable`))
  (bind _grapplecable_2 (`self.GrappleCable`))
  (bind _grappletargetlocation (`self.GrappleTargetLocation`))
  (bind _grapplecable_3 (`self.GrappleCable`))
  ;[0.5625 0.4396 0] Grapple Rope System
  (if Grappling
    (`SceneComponent.SetVisibility` _grapplecable true false)
    (set `CableComponent.bAttachEnd` true _grapplecable_2)
    (set `CableComponent.EndLocation` (`KismetMathLibrary.InverseTransformLocation` (`self.GetTransform`) _grappletargetlocation) _grapplecable_2)
    (set `CableComponent.CableLength` (/ (`KismetMathLibrary.Vector_Distance` _grappletargetlocation (`self.K2_GetActorLocation`)) 1.1) _grapplecable_2)
    (else
      (`SceneComponent.SetVisibility` _grapplecable false false)
      (set `CableComponent.bAttachEnd` false _grapplecable_3)
      (set `CableComponent.CableLength` 0.0 _grapplecable_3))))

(event `self.BeginSlideCameraTilt`
  ;[0.02543 0.176 0] Slide Camera Tilt
  (bind (_direction _cameratilt) (`Timeline|Timeline_1` :!label _label_3)
    (:`Update`
      (`self.SlideCameraTiltUpdate` _cameratilt))))

(event `self.EndSlideCameraTilt`
  ;[0.02543 0.176 0] Slide Camera Tilt
  (goto _label_3 :!via `Reverse`))

(event `self.StartDashingCameraEffect`
  ;[0.02776 0.1885 0] Dashing Camera Effect
  (bind (_direction _fovscale) (`Timeline|Timeline_2` :!via `PlayFromStart` :!label _label_4)
    (:`Update`
      (`self.UpdateDashFOV` _fovscale))))

(event `self.EndDashingCameraEffect`
  ;[0.02776 0.1885 0] Dashing Camera Effect
  (goto _label_4 :!via `Stop`))

(fn `UserConstructionScript`)